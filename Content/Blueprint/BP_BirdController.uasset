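; Player controller for a Flappy Bird-style game that makes the bird flap on left click.
; On BeginPlay it casts player character 0 to BP_FlappingBirdCharacter and caches the reference.
; Each click zeroes the capsule's physics velocity, then applies a fixed upward impulse, so every flap starts from rest.
; Yaw-relative forward and right movement-input nodes remain in the graph but never run.
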(event EventBeginPlay
  (bind _asbp_flapping_bird_character (Utilities|Casting|CastToBP_FlappingBirdCharacter (Game|GetPlayerCharacter 0)))
  (Variables|Default|SetAs%20BP%20Flapping%20Bird%20Character _asbp_flapping_bird_character))

(event Input|ActionEvents|InputActionLeftClick
  (params (Key :type Key%20Structure :default "None"))
  (bind _as_bp_flapping_bird_character (Variables|Default|GetAs%20BP%20Flapping%20Bird%20Character))
  (bind _capsulecomponent (Variables|/Script/Engine.Character|GetCapsuleComponent _as_bp_flapping_bird_character))
  (:Pressed
    (Physics|SetPhysicsLinearVelocity _capsulecomponent "0, 0, 0" false "None")
    (Physics|AddImpulse _capsulecomponent "0.000000,0.000000,500.000000" "None" false)))

(fn ConstructionScript)